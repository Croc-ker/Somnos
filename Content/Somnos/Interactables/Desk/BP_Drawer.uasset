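; BP_Drawer is an interactable desk drawer that slides open and shut and periodically stocks itself with random items.
; A looping timer gives a random chance to spawn an actor from AvailableItems, attached to Holder, only while the drawer is closed and holds no valid item.
; Use flip-flops a timeline that moves the Cube along local Y, updating the Open flag when the motion finishes.
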(event Custom|SpawnItem
  (if (and (and (== (Math|Random|RandomIntegerinRange 0 5) 0) (not (Variables|Default|GetOpen))) (not (Utilities|IsValid (Variables|Default|GetItem))))
    (bind _returnvalue (Game|SpawnActorfromClass (.OutItem (Utilities|Array|Random (Variables|Default|GetAvailableItems))) (Transformation|GetWorldTransform (Variables|Default|GetHolder)) "Undefined" "MultiplyWithRoot" 0 0))
    (Variables|Default|SetItem _returnvalue)
    (Transformation|AttachComponentToComponent _returnvalue (Variables|Default|GetHolder) "None" "SnapToTarget" "SnapToTarget" "KeepRelative" true)))

(event EventBeginPlay
  (Utilities|Time|SetTimerbyEvent (delegate Custom|SpawnItem) 3.0 true))

(event Collision|EventActorBeginOverlap
  (params (OtherActor :type Actor%20Object%20Reference)))

(event EventTick
  (params (DeltaSeconds :type Float%20%28single-precision%29)))

(event EventUse
  (bind _isa (Utilities|FlowControl|FlipFlop)
    (:A
      (bind _track (Timeline|Timeline Play)
        (:Update
          (Transformation|SetRelativeLocation (Variables|Default|GetCube) (Math|Vector|Lerp(Vector) "0, 0, 0" "0.000000,250.000000,0.000000" _track) false false))
        (:Finished
          (Variables|Default|SetOpen _isa))))
    (:B
      (Timeline|Timeline Reverse))))

(fn ConstructionScript)