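; BP_Computer is an interactable, possessable computer that the player controls through a movable cursor.
; Use switches possession from the current pawn to the computer, whose possession event replaces the Somnos input mapping context with the computer one.
; Look input slides the cursor on the world Y/Z axes with sweep, so collision can block it.
; The exit action re-possesses the first BP_Somnos found in the level.
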(event Input|EnhancedActionEvents|EnhancedInputActionIA_Look
  (params (ActionValue :type Vector%202D%20Structure) (ElapsedSeconds :type Float%20%28double-precision%29) (TriggeredSeconds :type Float%20%28double-precision%29) (InputAction :type Input%20Action%20Object%20Reference :default "/Game/Somnos/Input/Somnos/IA_Look.IA_Look"))
  (Transformation|AddWorldOffset (Variables|Default|GetCursor) (Math|Vector|MakeVector 0.0 (.x ActionValue) (.y ActionValue)) true false))

(event Input|EnhancedActionEvents|EnhancedInputActionIA_Exit
  (params (ActionValue :type Boolean) (ElapsedSeconds :type Float%20%28double-precision%29) (TriggeredSeconds :type Float%20%28double-precision%29) (InputAction :type Input%20Action%20Object%20Reference :default "/Game/Somnos/Input/Somnos/IA_Exit.IA_Exit"))
  (bind _returnvalue (Game|GetPlayerController 0))
  (Pawn|UnPossess _returnvalue)
  (bind _outactors (Actor|GetAllActorsOfClass "/Game/Somnos/Player/BP_Somnos.BP_Somnos_C"))
  (Pawn|Possess _returnvalue (Utilities|Array|Get(acopy) _outactors)))

(event EventUse
  (bind _returnvalue (Game|GetPlayerController 0))
  (Pawn|UnPossess _returnvalue)
  (Pawn|Possess _returnvalue self))

(event EventPossessed
  (params (NewController :type Controller%20Object%20Reference))
  (bind _assomnos_controller (Utilities|Casting|CastToSomnosController NewController))
  (Input|RemoveMappingContext (PlayerController|LocalPlayerSubsystems|GetEnhancedInputLocalPlayerSubsystem _assomnos_controller) "/Game/Somnos/Input/Somnos/IMC_Somnos.IMC_Somnos" "(bIgnoreAllPressedKeysUntilRelease=True,bForceImmediately=False,bNotifyUserSettings=False)")
  (Input|AddMappingContext (PlayerController|LocalPlayerSubsystems|GetEnhancedInputLocalPlayerSubsystem _assomnos_controller) "/Game/Somnos/Input/Computer/IMC_Computer.IMC_Computer" 0 "(bIgnoreAllPressedKeysUntilRelease=True,bForceImmediately=False,bNotifyUserSettings=False)"))

(fn ConstructionScript)