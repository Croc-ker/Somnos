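; BP_GunPlacement is an interactable that puts the gun back at its starting spot and takes it away from the player.
; On BeginPlay it finds the BP_Gun actor in the level and caches its transform.
; Its Use event detaches the gun, restores that cached transform and clears HasGun on the BP_Somnos player character.
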(event EventBeginPlay
  (bind _returnvalue (Actor|GetActorOfClass "/Game/Somnos/Interactables/Gun/BP_Gun.BP_Gun_C"))
  (bind _output_get (Variables|Default|SetGun _returnvalue))
  (Variables|Default|SetGunTransform (Transformation|GetActorTransform _output_get)))

(event Collision|EventActorBeginOverlap
  (params (OtherActor :type Actor%20Object%20Reference)))

(event EventTick
  (params (DeltaSeconds :type Float%20%28single-precision%29)))

(event EventUse
  (bind _gun (Variables|Default|GetGun))
  (Transformation|DetachFromActor _gun "KeepWorld" "KeepWorld" "KeepWorld")
  (Transformation|SetActorTransform _gun (Variables|Default|GetGunTransform))
  (bind _asbp_somnos (Utilities|Casting|CastToBP_Somnos (Game|GetPlayerCharacter 0)))
  (Variables|/Game/Somnos/Player/BP_Somnos.BP_Somnos_C|SetHasGun _asbp_somnos false))

(fn ConstructionScript)