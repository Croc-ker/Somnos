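; BP_Mirror is a usable mirror item in Somnos that the player picks up to see whether their character is sleeping.
; The first Use sets it as BP_Somnos's HeldItem, snaps it to the ItemHold component and sets its TextRender from IsSleeping, read only at that moment.
; A FlipFlop makes the second Use clear HeldItem, detach the mirror and destroy it rather than drop it.
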(event EventBeginPlay)

(event Collision|EventActorBeginOverlap
  (params (OtherActor :type Actor%20Object%20Reference)))

(event EventTick
  (params (DeltaSeconds :type Float%20%28single-precision%29)))

(event EventUse
  (bind _asbp_somnos (Utilities|Casting|CastToBP_Somnos (Game|GetPlayerCharacter 0)))
  (Utilities|FlowControl|FlipFlop
    (:A
      (Variables|/Game/Somnos/Player/BP_Somnos.BP_Somnos_C|SetHeldItem _asbp_somnos self)
      (Transformation|AttachComponentToComponent (Variables|/Game/Somnos/Player/BP_Somnos.BP_Somnos_C|GetItemHold _asbp_somnos) "None" "SnapToTarget" "SnapToTarget" "KeepRelative" true)
      (Rendering|Components|TextRender|SetText (Variables|Default|GetTextRender) (Utilities|String|SelectText "sleep :(" "no sleep :)" (Variables|/Game/Somnos/Player/BP_Somnos.BP_Somnos_C|GetIsSleeping _asbp_somnos))))
    (:B
      (Variables|/Game/Somnos/Player/BP_Somnos.BP_Somnos_C|SetHeldItem _asbp_somnos 0)
      (Transformation|DetachFromActor "KeepWorld" "KeepWorld" "KeepWorld")
      (Actor|DestroyActor))))

(fn ConstructionScript)