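; BP_Somnos is the player pawn, with a mouse-aimed held gun, health and a sleep mechanic.
; Interact fires at the cursor trace target or the player when self-aiming, or uses the target when unarmed.
; A looping timer builds toward sleep, and player-inflicted damage while asleep wakes the pawn and refunds ammo.
; Five peek inputs drive camera timelines, with peek and sleep changes broadcast to actors through interfaces.
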(event Custom|AddSleep
  (bind _result (Math|Float|IncrementFloat (Variables|Default|GetCurrentSleep))
    (:%20%20
      (if (>= _result (Variables|Default|GetSleepThreshold))
        (CallFunction|DoSleep true)))))

(event Input|EnhancedActionEvents|EnhancedInputActionIA_AimSelf
  (params (ActionValue :type Boolean) (ElapsedSeconds :type Float%20%28double-precision%29) (TriggeredSeconds :type Float%20%28double-precision%29) (InputAction :type Input%20Action%20Object%20Reference :default "/Game/Somnos/Input/Somnos/IA_AimSelf.IA_AimSelf"))
  (bind _camera (Variables|Default|GetCamera))
  (:Triggered
    (Variables|Default|SetLookAtLocation (Transformation|GetWorldLocation _camera))
    (Variables|Default|SetHandT (Math|Transform|MakeTransform (Math|Transform|InverseTransformLocation (Transformation|GetWorldTransform _camera) (+ (.location (Transformation|GetWorldTransform _camera)) "-5.000000,0.000000,-10.000000")) "120.000000,0.000000,0.000000")))
  (:Started
    (Variables|Default|SetAimSelf true))
  (:Canceled
    (Variables|Default|SetAimSelf false :!label _label))
  (:Completed
    (goto _label)))

(event Input|EnhancedActionEvents|EnhancedInputActionIA_PeekUp
  (params (ActionValue :type Boolean) (ElapsedSeconds :type Float%20%28double-precision%29) (TriggeredSeconds :type Float%20%28double-precision%29) (InputAction :type Input%20Action%20Object%20Reference :default "/Game/Somnos/Input/Somnos/IA_PeekUp.IA_PeekUp"))
  (:Started
    (Utilities|GetPeek "Up" :!label _label
      (:IsEmpty
        _)
      (:IsPeekName
        _))
    (Utilities|SetGargActions 0 "Up"
      (:Play
        (CallFunction|DoPeek true "Up")
        (bind _track (Timeline|PeekUp Play)
          (:Update
            (Transformation|SetRelativeTransform (Variables|Default|GetCamRoot) (Utilities|PeekLerp _track (Math|Transform|MakeTransform "85.000000,0.000000,75.000000" "0, 0, 0" "1.000000,1.000000,1.000000")) false false))))
      (:Reverse
        (CallFunction|DoPeek false "None")
        (Timeline|PeekUp Reverse))))
  (:Completed
    (goto _label Completed)))

(event Input|EnhancedActionEvents|EnhancedInputActionIA_PeekUnder
  (params (ActionValue :type Boolean) (ElapsedSeconds :type Float%20%28double-precision%29) (TriggeredSeconds :type Float%20%28double-precision%29) (InputAction :type Input%20Action%20Object%20Reference :default "/Game/Somnos/Input/Somnos/IA_PeekUnder.IA_PeekUnder"))
  (:Started
    (Utilities|GetPeek "Down" :!label _label
      (:IsEmpty
        _)
      (:IsPeekName
        _))
    (Utilities|SetGargActions 1 "Down"
      (:Play
        (CallFunction|DoPeek true "Down")
        (bind _track (Timeline|PeekUnder Play)
          (:Update
            (Transformation|SetRelativeTransform (Variables|Default|GetCamRoot) (Utilities|PeekLerp _track (Math|Transform|MakeTransform "-55.000000,10.000000,-60.000000" "-25.000000,2.000000,25.000000" "1.000000,1.000000,1.000000")) false false))))
      (:Reverse
        (CallFunction|DoPeek false "None")
        (Timeline|PeekUnder Reverse))))
  (:Completed
    (goto _label Completed)))

(event Input|EnhancedActionEvents|EnhancedInputActionIA_PeekLeft
  (params (ActionValue :type Boolean) (ElapsedSeconds :type Float%20%28double-precision%29) (TriggeredSeconds :type Float%20%28double-precision%29) (InputAction :type Input%20Action%20Object%20Reference :default "/Game/Somnos/Input/Somnos/IA_PeekLeft.IA_PeekLeft"))
  (:Started
    (Utilities|GetPeek "Left" :!label _label
      (:IsEmpty
        _)
      (:IsPeekName
        _))
    (Utilities|SetGargActions 3 "Left"
      (:Play
        (CallFunction|DoPeek true "Left")
        (bind _track (Timeline|PeekLR Play)
          (:Update
            (Transformation|SetRelativeTransform (Variables|Default|GetCamRoot) (Utilities|PeekLerp _track (Math|Transform|MakeTransform "0.000000,10.000000,0.000000" "45.000000,-160.000000,12.000000" "1.000000,1.000000,1.000000")) false false))))
      (:Reverse
        (CallFunction|DoPeek false "None")
        (Timeline|PeekLR Reverse))))
  (:Completed
    (goto _label Completed)))

(event Input|EnhancedActionEvents|EnhancedInputActionIA_PeekRight
  (params (ActionValue :type Boolean) (ElapsedSeconds :type Float%20%28double-precision%29) (TriggeredSeconds :type Float%20%28double-precision%29) (InputAction :type Input%20Action%20Object%20Reference :default "/Game/Somnos/Input/Somnos/IA_PeekRight.IA_PeekRight"))
  (:Started
    (Utilities|GetPeek "Right" :!label _label
      (:IsEmpty
        _)
      (:IsPeekName
        _))
    (Utilities|SetGargActions 2 "Right"
      (:Play
        (CallFunction|DoPeek true "Right")
        (bind _track (Timeline|Timeline Play)
          (:Update
            (Transformation|SetRelativeTransform (Variables|Default|GetCamRoot) (Utilities|PeekLerp _track (Math|Transform|MakeTransform "75.000000,-10.000000,25.000000" "0.000000,85.000000,-12.000000" "1.000000,1.000000,1.000000")) false false))))
      (:Reverse
        (CallFunction|DoPeek false "None")
        (Timeline|Timeline Reverse))))
  (:Completed
    (goto _label Completed)))

(event Input|EnhancedActionEvents|EnhancedInputActionIA_Interact
  (params (ActionValue :type Boolean) (ElapsedSeconds :type Float%20%28double-precision%29) (TriggeredSeconds :type Float%20%28double-precision%29) (InputAction :type Input%20Action%20Object%20Reference :default "/Game/Somnos/Input/Somnos/IA_Interact.IA_Interact"))
  (bind _returnvalue (Game|GetPlayerController 0))
  (bind _returnvalue_2 (Game|GetPlayerController 0))
  (bind _ammo (Variables|Default|GetAmmo))
  (bind _itemhold (Variables|Default|GetItemHold))
  (bind (_worldlocation _worlddirection) (Game|Player|ConvertMouseLocationToWorldSpace _returnvalue))
  (bind _outhit (Collision|LineTraceByChannel _worldlocation (+ _worldlocation (* _worlddirection 1e+04)) "TraceTypeQuery1" true (Utilities|Array|MakeArray self) "None"))
  (if (Variables|Default|GetHasGun)
    (if (> _ammo 0)
      (bind _asactor (Utilities|Casting|CastToActor (Utilities|SelectObject self (.HitActor (Collision|BreakHitResult _outhit)) (Variables|Default|GetAimSelf))))
      (Game|Damage|ApplyDamage _asactor 1.0 _returnvalue_2 _returnvalue_2)
      (bind _result (Math|Integer|DecrementInt _ammo)
        (:%20%20
          (Development|PrintString (Utilities|String|ToString(Integer) _result))
          (bind _asbp_gun (Utilities|Casting|CastToBP_Gun (Variables|Default|GetHeldItem)))
          (Default|Shoot _asbp_gun)
          (Transformation|AddRelativeRotation _itemhold "50.000000,0.000000,0.000000" false false)
          (Transformation|AddRelativeLocation _itemhold "-10.000000,0.000000,5.000000" false false)))
      (else
        (Audio|PlaySoundatLocation "/Game/Somnos/Sounds/Effects/gun_dry.gun_dry" (Transformation|GetWorldLocation (Variables|Default|GetItemHold)) "0, 0, 0" 1.0 1.0 0.0 0 0 0 0)))
    (else
      (Class|BPIUsable|Use(Message) (.HitActor (Collision|BreakHitResult _outhit))))))

(event Input|EnhancedActionEvents|EnhancedInputActionIA_Desk
  (params (ActionValue :type Boolean) (ElapsedSeconds :type Float%20%28double-precision%29) (TriggeredSeconds :type Float%20%28double-precision%29) (InputAction :type Input%20Action%20Object%20Reference :default "/Game/Somnos/Input/Somnos/IA_Desk.IA_Desk"))
  (:Started
    (Utilities|GetPeek "Desk" :!label _label
      (:IsEmpty
        _)
      (:IsPeekName
        _))
    (Utilities|SetGargActions 4 "Desk"
      (:Play
        (CallFunction|DoPeek true "Desk")
        (bind _track (Timeline|Desk Play)
          (:Update
            (Transformation|SetRelativeTransform (Variables|Default|GetCamRoot) (Utilities|PeekLerp _track (Math|Transform|MakeTransform "-30.000000,0.000000,30.000000" "-50.000000,-70.000000,-15.000000" "1.000000,1.000000,1.000000")) false false))))
      (:Reverse
        (CallFunction|DoPeek false "None")
        (Timeline|Desk Reverse))))
  (:Completed
    (goto _label Completed)))

(event Game|Damage|EventAnyDamage
  (params (Damage :type Float%20%28single-precision%29) (DamageType :type Damage%20Type%20Object%20Reference) (InstigatedBy :type Controller%20Object%20Reference) (DamageCauser :type Actor%20Object%20Reference))
  (if (and (== (Game|GetPlayerController 0) InstigatedBy) (Variables|Default|GetIsSleeping))
    (CallFunction|DoSleep false)
    (Math|Integer|IncrementInt (Variables|Default|GetAmmo)
      (:%20%20
        (Development|PrintString "you awake")
        (Class|BPIUsable|Use(Message) (Variables|Default|GetHeldItem))))
    (else
      (bind _output_get (Variables|Default|SetHealth (- (Variables|Default|GetHealth) Damage)))
      (if (<= _output_get 0.0)
        (Game|QuitGame 0 "Quit" false)
        (else
          (Development|PrintString "YEOWCH!!!!"))))))

(event EventBeginPlay
  (Utilities|Time|SetTimerbyEvent (delegate Custom|AddSleep) 0.5 true)
  (Audio|Components|Audio|Play (Variables|Default|GetAmbience) 0.0))

(event EventPossessed
  (params (NewController :type Controller%20Object%20Reference))
  ;[0.15 0.15 0.15 0.5] Input Mapping Context
  (bind _assomnos_controller (Utilities|Casting|CastToSomnosController NewController))
  (Input|AddMappingContext (PlayerController|LocalPlayerSubsystems|GetEnhancedInputLocalPlayerSubsystem _assomnos_controller) "/Game/Somnos/Input/Somnos/IMC_Somnos.IMC_Somnos" 1 "(bIgnoreAllPressedKeysUntilRelease=True,bForceImmediately=False,bNotifyUserSettings=False)")
  (Variables|/Script/Engine.PlayerController|SetbShowMouseCursor _assomnos_controller true)
  (Class|WidgetBlueprintLibrary|SetFocustoGameViewport))

(event EventTick
  (params (DeltaSeconds :type Float%20%28single-precision%29))
  (bind _returnvalue (Game|GetPlayerController 0))
  (bind _itemholdroot (Variables|Default|GetItemHoldRoot))
  (bind (_worldlocation _worlddirection) (Game|Player|ConvertMouseLocationToWorldSpace _returnvalue))
  (bind _returnvalue_2 (Transformation|GetWorldTransform _itemholdroot))
  (bind _outhit (Collision|LineTraceByChannel _worldlocation (+ _worldlocation (* _worlddirection 1e+04)) "TraceTypeQuery1" true (Utilities|Array|MakeArray self) "None"))
  (CallFunction|SetHeldItemTransform (Variables|Default|GetHandT))
  (Variables|Default|SetHandT (Math|Transform|MakeTransform (Math|Vector|MakeVector 0.0 (.y (/ (Math|Transform|InverseTransformLocation _returnvalue_2 (Variables|Default|GetLookAtLocation)) 3e+02)) (/ (.z (/ (Math|Transform|InverseTransformLocation _returnvalue_2 (Variables|Default|GetLookAtLocation)) 3e+02)) 1.5)) (Math|Transform|InverseTransformRotation _returnvalue_2 (Math|Rotator|FindLookatRotation (Transformation|GetWorldLocation (Variables|Default|GetItemHold)) (Variables|Default|GetLookAtLocation)))))
  (Variables|Default|SetLookAtLocation (.TraceEnd (Collision|BreakHitResult _outhit))))

(event Input|KeyboardEvents|DebugKeyM
  (params (Key :type Key%20Structure :default "None") (ActionValue :type Input%20Action%20Value%20Structure))
  (:Pressed
    (Game|Damage|ApplyDamage self -1.0 0 0)
    (Math|Integer|IncrementInt (Variables|Default|GetAmmo))))

(event Input|KeyboardEvents|DebugKeyC
  (params (Key :type Key%20Structure :default "None") (ActionValue :type Input%20Action%20Value%20Structure))
  (:Pressed
    (CallFunction|DoSleep true)))

(event Input|KeyboardEvents|DebugKeyT
  (params (Key :type Key%20Structure :default "None") (ActionValue :type Input%20Action%20Value%20Structure))
  (:Pressed
    (Class|BPIUsable|Use(Message) (Variables|Default|GetHeldItem))))

(fn ConstructionScript)

(fn DoSleep
  (params (IsSleep :type Boolean))
  (bind _outactors (Actor|GetAllActorswithInterface "/Game/Somnos/Interactables/BPI_SleepBased.BPI_SleepBased_C"))
  (for _array_element _outactors
    (Class|BPISleepBased|OnSleep(Message) _array_element IsSleep))
  (Variables|Default|SetIsSleeping IsSleep)
  (Variables|Default|SetCurrentSleep 0.0))

(fn SetHeldItemTransform
  (params (Relative%20Transform :type Transform))
  (Transformation|SetRelativeTransform (Variables|Default|GetItemHold) (Class|KismetMathLibrary|TInterpto (Transformation|GetRelativeTransform (Variables|Default|GetItemHold)) Relative%20Transform (Utilities|Time|GetWorldDeltaSeconds) 4.0) false false))

(fn FinishTask)

(fn DoPeek
  (params (IsPeeking :type Boolean) (Peek :type Name))
  (bind _outactors (Actor|GetAllActorswithInterface "/Game/Somnos/Interactables/BPI_PeekBased.BPI_PeekBased_C"))
  (for _array_element _outactors
    (Class|BPIPeekBased|OnPeek(Message) _array_element IsPeeking Peek)))