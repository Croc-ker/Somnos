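; Spawner that keeps one Skinhost enemy in play, respawning it at its own transform whenever none exists.
; A fast looping timer checks for a valid Skinhost and a clear Peeking flag, then waits a random 30–60 second Delay before spawning.
; The new AI receives a reference back to this spawner, and the OnPeek event sets the flag that blocks new spawn countdowns.
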(event Custom|Respawn
  (bind _returnvalue (Transformation|GetActorTransform))
  (if (not (or (Utilities|IsValid (Variables|Default|GetSkinhost)) (Variables|Default|GetPeeking)))
    (Utilities|FlowControl|Delay (Math|Random|RandomFloatinRange 3e+01 6e+01))
    (bind _returnvalue_2 (AI|SpawnAIFromClass "/Game/Somnos/Enemies/Skinhost/BP_Skinhost.BP_Skinhost_C" 0 (.location _returnvalue) (.rotation _returnvalue) false 0))
    (bind _asbp_skinhost (Utilities|Casting|CastToBP_Skinhost _returnvalue_2))
    (bind _output_get (Variables|Default|SetSkinhost _asbp_skinhost))
    (Variables|/Game/Somnos/Enemies/Skinhost/BP_Skinhost.BP_Skinhost_C|SetSpawner _output_get self)))

(event EventBeginPlay
  (bind _asbp_somnos (Utilities|Casting|CastToBP_Somnos (Game|GetPlayerCharacter 0)))
  (Variables|Default|SetPlayer _asbp_somnos)
  (Utilities|Time|SetTimerbyEvent (delegate Custom|Respawn) 0.1 true true))

(event EventOnPeek
  (params (IsPeeking :type Boolean) (Peek :type Name :default "None"))
  (Variables|Default|SetPeeking IsPeeking))

(fn ConstructionScript)