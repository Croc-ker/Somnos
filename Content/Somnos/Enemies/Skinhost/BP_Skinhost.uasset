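; BP_Skinhost is the Skinhost enemy Blueprint in Somnos, holding minimal reactions to being shot and to peek events.
; OnShot destroys the actor immediately, and OnPeek stores the incoming Peek value without acting on it here.
; BeginPlay and the construction script only call their parents, while Tick and overlap events are disabled.
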(event EventBeginPlay
  (|CallParentFunction))

(event Collision|EventActorBeginOverlap
  (params (OtherActor :type Actor%20Object%20Reference))
  (|CallParentFunction OtherActor) ; This node is disabled and will not be called.\nDrag off pins to build functionality.
)

(event EventTick
  (params (DeltaSeconds :type Float%20%28single-precision%29))
  (|CallParentFunction DeltaSeconds) ; This node is disabled and will not be called.\nDrag off pins to build functionality.
)

(event EventOnShot
  (Actor|DestroyActor))

(event EventOnPeek
  (params (IsPeeking :type Boolean) (Peek :type Name :default "None"))
  (Variables|Default|SetPeek Peek))

(fn ConstructionScript
  (|CallParentFunction))